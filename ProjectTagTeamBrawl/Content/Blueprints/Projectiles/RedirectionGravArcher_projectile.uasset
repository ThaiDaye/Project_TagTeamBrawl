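; Spinning Grav Archer projectile that damages enemies inside its box and redirects other projectiles passing through it.
; A looping timer deals chip damage and stagger to overlapping enemies, while a timeline eases its velocity up from zero.
; When a Projectile_MASTER enters the box, sphere and line traces gather nearby enemies in its line of sight into Targets.
; The projectile turns toward a random target at double base speed with knockup enabled.
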(event OnComponentBeginOverlap(Box)
  (params (OverlappedComponent :type Primitive%20Component%20Object%20Reference) (OtherActor :type Actor%20Object%20Reference) (OtherComp :type Primitive%20Component%20Object%20Reference) (OtherBodyIndex :type Integer) (bFromSweep :type Boolean) (SweepResult :type Hit%20Result%20Structure%20%28by%20ref%29))
  (bind _returnvalue (Transformation|GetActorLocation))
  (bind _targets (Variables|Default|GetTargets))
  (bind _asprojectile_master (Utilities|Casting|CastToProjectile_MASTER OtherActor))
  (bind _output_get (Variables|Default|SetAs%20Projectile%20MASTER _asprojectile_master))
  (bind _outhits (Collision|MultiSphereTraceForObjects _returnvalue _returnvalue 1e+03 (Utilities|Array|MakeArray "ObjectTypeQuery3" "ObjectTypeQuery1" "ObjectTypeQuery2") false 0 "None"))
  (for _array_element _outhits
    (bind _asenemy_character (Utilities|Casting|CastToEnemy_Character (.HitActor (Collision|BreakHitResult _array_element))))
    (bind _outhit (Collision|LineTraceForObjects (Transformation|GetActorLocation _output_get) (Transformation|GetActorLocation _asenemy_character) (Utilities|Array|MakeArray "ObjectTypeQuery2" "ObjectTypeQuery1") false 0 "None"))
    (if (not (.bBlockingHit (Collision|BreakHitResult _outhit)))
      (Utilities|Array|Add (Variables|Default|GetTargets) _asenemy_character)))
  (bind _output_get_2 (Variables|Default|SetTargetRef (Utilities|Array|Get(acopy) _targets (Math|Random|RandomIntegerinRange 0 (Utilities|Array|Length _targets)))))
  (Utilities|IsValid _output_get_2
    (:Is%20Valid
      (Utilities|IsValid _output_get
        (:Is%20Valid
          (Transformation|SetActorRotation _output_get (Math|Rotator|MakeRotator 0.0 0.0 (.yaw (Math|Rotator|FindLookatRotation (Transformation|GetActorLocation _output_get) (Transformation|GetActorLocation (Variables|Default|GetTargetRef))))))
          (Variables|/Game/Blueprints/MASTERS/Projectile_MASTER.Projectile_MASTER_C|SetVelocity _output_get (* (Variables|/Game/Blueprints/MASTERS/Projectile_MASTER.Projectile_MASTER_C|GetBaseVelocity _output_get) 2.0))
          (Variables|/Game/Blueprints/MASTERS/Projectile_MASTER.Projectile_MASTER_C|SetKnockup _output_get true))))))

(event Custom|TickDamage
  (bind _returnvalue (Transformation|GetActorLocation))
  (for _array_element (Collision|GetOverlappingActors (Variables|Default|GetBox) "/Game/Blueprints/Enemies/Enemy_Character.Enemy_Character_C" :!class /Script/Engine.PrimitiveComponent)
    (Utilities|IsValid _array_element
      (:Is%20Valid
        (Default|RecieveDamage (.AsEnemy%20Character (Utilities|Casting|CastToEnemy_Character _array_element)) (Variables|Default|GetProjectile%20Damage) (Math|Rotator|GetRotationXVector (Math|Rotator|FindLookatRotation (Math|Vector|MakeVector (.x _returnvalue) (.y _returnvalue) 0.0) (Math|Vector|MakeVector (.x (Transformation|GetActorLocation _array_element)) (.y (Transformation|GetActorLocation _array_element)) 0.0))) (Variables|Default|GetProjectile%20Stagger) false true (Transformation|GetActorLocation (.AsEnemy%20Character (Utilities|Casting|CastToEnemy_Character _array_element))) false false false)))))

(event EventBeginPlay
  (|CallParentFunction)
  (Utilities|FlowControl|Sequence
    (:then_0
      (Utilities|FlowControl|Delay 0.2)
      (Utilities|Time|SetTimerbyEvent (delegate Custom|TickDamage) 0.1 true))
    (:then_1
      (bind _newtrack_0 (Timeline|Timeline_0 PlayFromStart)
        (:Update
          (Variables|Default|SetVelocity (Math|Float|Lerp 0.0 2.0 _newtrack_0)))))))

(event EventTick
  (params (DeltaSeconds :type Float%20%28single-precision%29))
  (Transformation|AddLocalRotation (Variables|Default|GetStaticMesh) "0.000000,5.000000,0.000000" false false))

(fn ConstructionScript
  (|CallParentFunction))