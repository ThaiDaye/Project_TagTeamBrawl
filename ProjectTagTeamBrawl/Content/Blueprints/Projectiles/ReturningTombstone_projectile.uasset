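; Returning tombstone projectile that flies back to the player, spinning and damaging enemies along the way.
; On BeginPlay a timeline lerps it from its spawn location toward the player's live position, then calls TombstoneReturned on the player and destroys itself.
; A looping timer repeatedly applies damage and stagger to enemies overlapping its box, with hit direction pointing away from the projectile.
; Tick rotates the mesh for the spin.
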(event Custom|TickDamage
  (bind _returnvalue (Transformation|GetActorLocation))
  (for _array_element (Collision|GetOverlappingActors (Variables|Default|GetBox) "/Game/Blueprints/Enemies/Enemy_Character.Enemy_Character_C" :!class /Script/Engine.PrimitiveComponent)
    (Utilities|IsValid _array_element
      (:Is%20Valid
        (Default|RecieveDamage (.AsEnemy%20Character (Utilities|Casting|CastToEnemy_Character _array_element)) (Variables|Default|GetProjectile%20Damage) (Math|Rotator|GetRotationXVector (Math|Rotator|FindLookatRotation (Math|Vector|MakeVector (.x _returnvalue) (.y _returnvalue) 0.0) (Math|Vector|MakeVector (.x (Transformation|GetActorLocation _array_element)) (.y (Transformation|GetActorLocation _array_element)) 0.0))) (Variables|Default|GetProjectile%20Stagger))))))

(event EventBeginPlay
  (|CallParentFunction)
  (bind _outactors (Actor|GetAllActorsOfClass "/Game/Blueprints/Player_Character.Player_Character_C"))
  (Variables|Default|SetPlayerRef (Utilities|Array|Get(acopy) _outactors))
  (Utilities|FlowControl|Sequence
    (:then_0
      (Utilities|Time|SetTimerbyEvent (delegate Custom|TickDamage) 0.15 true))
    (:then_1
      (Variables|Default|SetBeforeLocartion (Transformation|GetActorLocation))
      (bind _newtrack_0 (Timeline|Timeline_0 PlayFromStart)
        (:Update
          (Transformation|SetActorLocation (Math|Vector|Lerp(Vector) (Variables|Default|GetBeforeLocartion) (Transformation|GetActorLocation (Variables|Default|GetPlayerRef)) _newtrack_0) false false))
        (:Finished
          (Default|TombstoneReturned (Variables|Default|GetPlayerRef))
          (Actor|DestroyActor))))))

(event EventTick
  (params (DeltaSeconds :type Float%20%28single-precision%29))
  (Transformation|AddLocalRotation (Variables|Default|GetStaticMesh) "-20.000000, 0,0.000000" false false))

(fn ConstructionScript
  (|CallParentFunction))