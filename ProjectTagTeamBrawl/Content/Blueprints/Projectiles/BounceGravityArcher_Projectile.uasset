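; Gravity archer projectile that bounces between nearby enemies, then hands off to a returning boomerang projectile.
; On BeginPlay it gathers enemies via a sphere trace, keeping those with no WorldDynamic line-trace hit.
; A timeline lerps it to each target in turn, dealing damage and stagger on arrival with short pauses between.
; After the last, it spawns BoomerangGravityArcher_Projectile facing the player and destroys itself; the TickDamage timer is unwired.
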(event Custom|TickDamage
  (bind _returnvalue (Transformation|GetActorLocation))
  (bind _returnvalue_2 (Transformation|GetActorLocation))
  (bind _box (Variables|Default|GetBox))
  (Utilities|IsValid _box
    (:Is%20Valid
      (for _array_element (Collision|GetOverlappingActors _box "/Game/Blueprints/Enemies/Enemy_Character.Enemy_Character_C" :!class /Script/Engine.PrimitiveComponent)
        (Utilities|IsValid _array_element
          (:Is%20Valid
            (Default|RecieveDamage (.AsEnemy%20Character (Utilities|Casting|CastToEnemy_Character _array_element)) (Variables|Default|GetProjectile%20Damage) (Math|Rotator|GetRotationXVector (Math|Rotator|FindLookatRotation (Math|Vector|MakeVector (.x _returnvalue) (.y _returnvalue) 0.0) (Math|Vector|MakeVector (.x (Transformation|GetActorLocation _array_element)) (.y (Transformation|GetActorLocation _array_element)) 0.0))) (Variables|Default|GetProjectile%20Stagger) (Variables|Default|GetCanKnockup) false (Transformation|GetActorLocation (.AsEnemy%20Character (Utilities|Casting|CastToEnemy_Character _array_element))))
            (if (> (Variables|/Game/Blueprints/Enemies/Enemy_Character.Enemy_Character_C|GetGravityArrowCount (.AsEnemy%20Character (Utilities|Casting|CastToEnemy_Character _array_element))) 0)
              (Collision|MultiSphereTraceForObjects _returnvalue_2 _returnvalue_2 7.5e+02 (Utilities|Array|MakeArray "ObjectTypeQuery3") false 0 "ForDuration" true "(R=1.000000,G=0.000000,B=0.000000,A=1.000000)" "(R=0.000000,G=1.000000,B=0.000000,A=1.000000)" 1.0))))))))

(event Custom|BounceBetweentargets
  (bind _returnvalue (Transformation|GetActorLocation))
  (bind _returnvalue_2 (Transformation|GetActorLocation))
  (bind _returnvalue_3 (Transformation|GetActorLocation))
  (bind _targets (Variables|Default|GetTargets))
  (bind _targets_2 (Variables|Default|GetTargets))
  (bind _returnvalue_4 (Utilities|Array|Length _targets_2))
  (bind _outhits (Collision|MultiSphereTraceForObjects _returnvalue _returnvalue 5e+02 (Utilities|Array|MakeArray "ObjectTypeQuery3") false 0 "None" true "(R=1.000000,G=0.000000,B=0.000000,A=1.000000)" "(R=0.000000,G=1.000000,B=0.000000,A=1.000000)" 1.0))
  (for _array_element _outhits
    (bind _asenemy_character (Utilities|Casting|CastToEnemy_Character (.HitActor (Collision|BreakHitResult _array_element))))
    (if (not (Utilities|Array|ContainsItem _targets _asenemy_character))
      (bind _outhit (Collision|LineTraceForObjects (Transformation|GetActorLocation) (Transformation|GetActorLocation _asenemy_character) (Utilities|Array|MakeArray "ObjectTypeQuery2") false 0 "None"))
      (if (not (.bBlockingHit (Collision|BreakHitResult _outhit)))
        (Utilities|Array|Add _targets _asenemy_character))))
  (bind _output_get (Variables|Default|SetBeforeLocation _returnvalue_3 :!label _label))
  (bind _newtrack_0 (Timeline|Timeline_0 PlayFromStart)
    (:Update
      (Utilities|IsValid (Utilities|Array|Get(acopy) (Variables|Default|GetTargets) (Variables|Default|GetCurrentTarget))
        (:Is%20Valid
          (Transformation|SetActorLocation (Math|Vector|Lerp(Vector) (Variables|Default|GetBeforeLocation) (Transformation|GetActorLocation (Utilities|Array|Get(acopy) (Variables|Default|GetTargets) (Variables|Default|GetCurrentTarget))) _newtrack_0) false false))))
    (:Finished
      (Utilities|IsValid (Utilities|Array|Get(acopy) (Variables|Default|GetTargets) (Variables|Default|GetCurrentTarget))
        (:Is%20Valid
          (Default|RecieveDamage (Utilities|Array|Get(acopy) (Variables|Default|GetTargets) (Variables|Default|GetCurrentTarget)) 1.0 (Math|Rotator|GetRotationXVector (Math|Rotator|FindLookatRotation _output_get _returnvalue_3)) 1.5e+02 (Variables|Default|GetCanKnockup) false (Transformation|GetActorLocation (Utilities|Array|Get(acopy) (Variables|Default|GetTargets) (Variables|Default|GetCurrentTarget)))))
        (:Is%20Not%20Valid
          _))
      (bind _output_get_2 (Variables|Default|SetCurrentTarget (Math|Integer|Clamp(Integer) (+ (Variables|Default|GetCurrentTarget) 1) 0 _returnvalue_4)))
      (if (== _output_get_2 _returnvalue_4)
        (Utilities|FlowControl|Delay 0.5)
        (bind _returnvalue_5 (Game|SpawnActorfromClass "/Game/Blueprints/Projectiles/BoomerangGravityArcher_Projectile.BoomerangGravityArcher_Projectile_C" (Math|Transform|MakeTransform _returnvalue_2 (Math|Rotator|FindLookatRotation _returnvalue_2 (Transformation|GetActorLocation (Variables|Default|GetPlayerRef)))) "AlwaysSpawn" 0 true 1.0 1.0 75.0 3.0 (Variables|Default|GetCanKnockup) 0))
        (Actor|DestroyActor)
        (else
          (Utilities|FlowControl|Delay 0.25)
          (goto _label))))))

(event EventBeginPlay
  (|CallParentFunction)
  (CallFunction|BounceBetweentargets))

(fn ConstructionScript
  (|CallParentFunction))