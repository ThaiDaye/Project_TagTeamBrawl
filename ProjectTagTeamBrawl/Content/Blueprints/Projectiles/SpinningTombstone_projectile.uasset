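; Spinning tombstone projectile that damages enemies in its area, then plants itself as a tombstone entity.
; Tick spins the mesh while a timeline scales velocity from the base value.
; After a short delay, a looping timer damages, staggers and optionally knocks up overlapping enemies, pushing away from the projectile.
; A second timer traces down to the ground, spawns StaticEntity_Tombstone at the impact point and destroys the projectile.
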(event Custom|TickDamage
  (bind _returnvalue (Transformation|GetActorLocation))
  (for _array_element (Collision|GetOverlappingActors (Variables|Default|GetBox) "/Game/Blueprints/Enemies/Enemy_Character.Enemy_Character_C" :!class /Script/Engine.PrimitiveComponent)
    (Utilities|IsValid _array_element
      (:Is%20Valid
        (Default|RecieveDamage (.AsEnemy%20Character (Utilities|Casting|CastToEnemy_Character _array_element)) (Variables|Default|GetProjectile%20Damage) (Math|Rotator|GetRotationXVector (Math|Rotator|FindLookatRotation (Math|Vector|MakeVector (.x _returnvalue) (.y _returnvalue) 0.0) (Math|Vector|MakeVector (.x (Transformation|GetActorLocation _array_element)) (.y (Transformation|GetActorLocation _array_element)) 0.0))) (Variables|Default|GetProjectile%20Stagger) (Variables|Default|GetCanKnockup) false (Transformation|GetActorLocation (.AsEnemy%20Character (Utilities|Casting|CastToEnemy_Character _array_element))) false false false)))))

(event Custom|Plant
  (bind _box (Variables|Default|GetBox))
  (bind _returnvalue (Transformation|GetWorldLocation _box))
  (bind _outhit (Collision|LineTraceForObjects _returnvalue (+ _returnvalue "0, 0,-10000.000000") (Utilities|Array|MakeArray "ObjectTypeQuery1" "ObjectTypeQuery2") false 0 "None"))
  (Game|SpawnActorfromClass "/Game/Blueprints/StaticEntities/StaticEntity_Tombstone.StaticEntity_Tombstone_C" (Math|Transform|MakeTransform (.ImpactPoint (Collision|BreakHitResult _outhit))) "AlwaysSpawn" 0 0)
  (Actor|DestroyActor))

(event EventBeginPlay
  (|CallParentFunction)
  (Utilities|FlowControl|Sequence
    (:then_0
      (Utilities|FlowControl|Delay 0.2)
      (Utilities|Time|SetTimerbyEvent (delegate Custom|TickDamage) 0.3 true))
    (:then_1
      (Utilities|Time|SetTimerbyEvent (delegate Custom|Plant) 2.0)
      (bind _newtrack_0 (Timeline|Timeline_0 PlayFromStart)
        (:Update
          (Variables|Default|SetVelocity (Math|Float|Lerp 0.0 (Variables|Default|GetBaseVelocity) _newtrack_0)))))))

(event EventTick
  (params (DeltaSeconds :type Float%20%28single-precision%29))
  (Transformation|AddLocalRotation (Variables|Default|GetStaticMesh) "20.000000, 0,0.000000" false false))

(fn ConstructionScript
  (|CallParentFunction))