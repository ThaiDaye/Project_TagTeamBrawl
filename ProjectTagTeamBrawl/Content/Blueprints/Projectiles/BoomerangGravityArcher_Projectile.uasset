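; Boomerang projectile for the gravity archer that flies out, returns to the player and is destroyed on getting close.
; A timeline reverses velocity unless it starts returning; hitting a surface forces an early return.
; While returning, a looping timer keeps it aligned to the player and ignores WorldDynamic collision.
; Another timer damages overlapping enemies, swapping it for a BounceGravityArcher projectile if the last one has gravity arrows.
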(event Custom|TickDamage
  (bind _returnvalue (Transformation|GetActorLocation))
  (bind _box (Variables|Default|GetBox))
  (Utilities|IsValid _box
    (:Is%20Valid
      (for _array_element (Collision|GetOverlappingActors _box "/Game/Blueprints/Enemies/Enemy_Character.Enemy_Character_C" :!class /Script/Engine.PrimitiveComponent)
        (bind _ascharacter_master (Utilities|Casting|CastToCharacter_MASTER _array_element))
        (Utilities|IsValid _array_element
          (:Is%20Valid
            (Default|RecieveDamage _ascharacter_master (Variables|Default|GetProjectile%20Damage) (Math|Rotator|GetRotationXVector (Math|Rotator|FindLookatRotation (Math|Vector|MakeVector (.x _returnvalue) (.y _returnvalue) 0.0) (Math|Vector|MakeVector (.x (Transformation|GetActorLocation _array_element)) (.y (Transformation|GetActorLocation _array_element)) 0.0))) (Variables|Default|GetProjectile%20Stagger) (Variables|Default|GetCanKnockup) false (Transformation|GetActorLocation _ascharacter_master) false))))
      (bind _asenemy_character (Utilities|Casting|CastToEnemy_Character _array_element))
      (if (> (Variables|/Game/Blueprints/Enemies/Enemy_Character.Enemy_Character_C|GetGravityArrowCount _asenemy_character) 0)
        (Game|SpawnActorfromClass "/Game/Blueprints/Projectiles/BounceGravityArcher_Projectile.BounceGravityArcher_Projectile_C" (Transformation|GetActorTransform) "AlwaysSpawn" 0 0.0 0.0 75.0 5.0 (Variables|Default|GetCanKnockup) 0)
        (Actor|DestroyActor)))))

(event Custom|SetRot
  (bind _returnvalue (Transformation|GetActorRotation))
  (if (< (Variables|Default|GetVelocity) 0.0)
    (Collision|SetCollisionResponsetoChannel (Variables|Default|GetBox) "ECC_WorldDynamic" "ECR_Ignore")
    (if (< (Transformation|GetDistanceTo (Variables|Default|GetPlayerRef)) 1e+02)
      (Actor|DestroyActor)
      (else
        (Transformation|SetActorRotation (Math|Rotator|MakeRotator (.roll _returnvalue) (.pitch _returnvalue) (.yaw (Math|Rotator|FindLookatRotation (Transformation|GetActorLocation (Variables|Default|GetPlayerRef)) (Transformation|GetActorLocation)))))))
    (else
      (Collision|SetCollisionResponsetoChannel (Variables|Default|GetStaticMesh) "ECC_WorldDynamic" "ECR_Block"))))

(event EventBeginPlay
  (bind _basevelocity (Variables|Default|GetBaseVelocity))
  (|CallParentFunction)
  (Utilities|Time|SetTimerbyEvent (delegate Custom|SetRot) 0.001 true)
  (if (Variables|Default|GetReturn)
    (Utilities|FlowControl|Sequence
      (:then_0
        (if (Variables|Default|GetReturn) :!label _label
          (Variables|Default|SetVelocity (* (Variables|Default|GetVelocity) -1.0))
          (else
            (bind _newtrack_0 (Timeline|Timeline_0 PlayFromStart)
              (:Update
                (if (not (Variables|Default|GetHitSurfaceReturn))
                  (Variables|Default|SetVelocity (Math|Float|Lerp _basevelocity (* _basevelocity -1.0) _newtrack_0))))))))
      (:then_1
        (Utilities|FlowControl|Delay 0.2)
        (Utilities|Time|SetTimerbyEvent (delegate Custom|TickDamage) 0.1 true)))
    (else
      (Utilities|Time|SetTimerbyEvent (delegate Custom|TickDamage) 0.1 true)
      (goto _label))))

(event Collision|EventHit
  (params (MyComp :type Primitive%20Component%20Object%20Reference) (Other :type Actor%20Object%20Reference) (OtherComp :type Primitive%20Component%20Object%20Reference) (bSelfMoved :type Boolean) (HitLocation :type Vector :default "0, 0, 0") (HitNormal :type Vector :default "0, 0, 0") (NormalImpulse :type Vector :default "0, 0, 0") (Hit :type Hit%20Result%20Structure%20%28by%20ref%29))
  (|CallParentFunction MyComp Other OtherComp bSelfMoved HitLocation HitNormal NormalImpulse Hit)
  (Variables|Default|SetVelocity -1.0)
  (CallFunction|ReApplyVelocity)
  (Variables|Default|SetHitSurfaceReturn true))

(fn ConstructionScript
  (|CallParentFunction))