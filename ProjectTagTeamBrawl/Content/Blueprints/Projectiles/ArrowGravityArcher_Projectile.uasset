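; Gravity archer arrow projectile that limits how many gravity arrows can be active on one enemy.
; On hit, it runs parent logic, then increments the Enemy_Character's GravityArrowCount, or destroys itself if the enemy is dead or already at three.
; On destruction, it decrements the count on its PlantedTarget, using the ToomanYArrows flag to skip rejected arrows that were never counted.
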(event EventBeginPlay
  (|CallParentFunction))

(event Collision|EventHit
  (params (MyComp :type Primitive%20Component%20Object%20Reference) (Other :type Actor%20Object%20Reference) (OtherComp :type Primitive%20Component%20Object%20Reference) (bSelfMoved :type Boolean) (HitLocation :type Vector :default "0, 0, 0") (HitNormal :type Vector :default "0, 0, 0") (NormalImpulse :type Vector :default "0, 0, 0") (Hit :type Hit%20Result%20Structure%20%28by%20ref%29))
  (|CallParentFunction MyComp Other OtherComp bSelfMoved HitLocation HitNormal NormalImpulse Hit)
  (bind _asenemy_character (Utilities|Casting|CastToEnemy_Character Other))
  (if (>= (Variables|/Game/Blueprints/Enemies/Enemy_Character.Enemy_Character_C|GetGravityArrowCount _asenemy_character) 3)
    (Variables|Default|SetToomanYArrows true :!label _label)
    (Actor|DestroyActor)
    (elif (Variables|/Game/Blueprints/MASTERS/Character_MASTER.Character_MASTER_C|GetIsDead _asenemy_character)
      (goto _label)
      (else
        (Variables|/Game/Blueprints/Enemies/Enemy_Character.Enemy_Character_C|SetGravityArrowCount _asenemy_character (+ (Variables|/Game/Blueprints/Enemies/Enemy_Character.Enemy_Character_C|GetGravityArrowCount _asenemy_character) 1))))))

(event EventDestroyed
  (if (not (Variables|Default|GetToomanYArrows))
    (bind _asenemy_character (Utilities|Casting|CastToEnemy_Character (Variables|Default|GetPlantedTarget)))
    (Utilities|IsValid _asenemy_character
      (:Is%20Valid
        (Variables|/Game/Blueprints/Enemies/Enemy_Character.Enemy_Character_C|SetGravityArrowCount _asenemy_character (Math|Integer|Clamp(Integer) (- (Variables|/Game/Blueprints/Enemies/Enemy_Character.Enemy_Character_C|GetGravityArrowCount _asenemy_character) 1) 0 3))))))

(fn ConstructionScript
  (|CallParentFunction))