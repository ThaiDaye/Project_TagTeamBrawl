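; Enemy character that chases the player on foot and freezes during combat states.
; From BeginPlay, a loop sends AIMoveTo at the player when within range and unblocked by WorldDynamic objects, otherwise retrying after a delay.
; The loop resumes after a successful move, but a failed move ends it.
; Tick zeroes walk speed and disables movement while dealing damage, being hit, knocked up, staggered or dead, otherwise restoring walking.
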(event EventBeginPlay
  (|CallParentFunction)
  (bind _outactors (Actor|GetAllActorsOfClass "/Game/Blueprints/Player_Character.Player_Character_C"))
  (bind _output_get (Variables|Default|SetPlayerRef (Utilities|Array|Get(acopy) _outactors)))
  (bind _outhit (Collision|LineTraceForObjects (+ (Transformation|GetActorLocation) "0, 0,50.000000") (+ (Transformation|GetActorLocation (Variables|Default|GetPlayerRef)) "0, 0,50.000000") (Utilities|Array|MakeArray "ObjectTypeQuery2") false 0 "None" :!label _label))
  (if (and (<= (Transformation|GetDistanceTo (Variables|Default|GetPlayerRef)) 5e+02) (not (.bBlockingHit (Collision|BreakHitResult _outhit))))
    (AI|AIMoveTo self "0, 0, 0" _output_get 5e+01 false
      (:OnSuccess
        (Utilities|FlowControl|Delay 0.5)
        (goto _label)))
    (else
      (Utilities|FlowControl|Delay 5.0)
      (goto _label))))

(event Collision|EventActorBeginOverlap
  (params (OtherActor :type Actor%20Object%20Reference))
  (|CallParentFunction OtherActor) ; This node is disabled and will not be called.\nDrag off pins to build functionality.
)

(event EventTick
  (params (DeltaSeconds :type Float%20%28single-precision%29))
  (bind _charactermovement (Variables|Character|GetCharacterMovement))
  (bind _staggered (Variables|Default|GetStaggered))
  (bind _knockedup (Variables|Default|GetKnockedUp))
  (bind _beinghitindicator (Variables|Default|GetBeingHitIndicator))
  (bind _dealingdamageindicator (Variables|Default|GetDealingDamageIndicator))
  (bind _isdead (Variables|Default|GetIsDead))
  (bind _returnvalue (Math|Boolean|ORBoolean _dealingdamageindicator _beinghitindicator _knockedup _isdead _staggered))
  (|CallParentFunction DeltaSeconds)
  (Variables|/Script/Engine.CharacterMovementComponent|SetMaxWalkSpeed (Variables|Character|GetCharacterMovement) (Math|Float|Lerp (Variables|Default|GetWalkSpeed) 0.0 (Math|Conversions|ToFloat(Boolean) _returnvalue)))
  (if _returnvalue
    (Pawn|Components|CharacterMovement|DisableMovement _charactermovement)
    (else
      (Pawn|Components|CharacterMovement|SetMovementMode _charactermovement "MOVE_Walking" 0))))

(fn ConstructionScript
  (|CallParentFunction))