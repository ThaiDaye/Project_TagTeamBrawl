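; Melee enemy character that chases the player and strikes at close range.
; A looping walk-to chain after BeginPlay checks distance and line of sight, runs AI MoveTo, calls MeleeAttack on arrival, then retries after a delay.
; MeleeAttack uses a Gate as a cooldown, turns to face, winds up, rechecks hit-reaction states, then sphere-traces to deal damage and stagger to the player.
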(event Custom|MeleeAttack
  (bind _scene (Variables|Default|GetScene))
  (bind _returnvalue (Transformation|GetWorldLocation _scene))
  (if (not (Math|Boolean|ORBoolean (Variables|Default|GetBeingHitIndicator) (Variables|Default|GetKnockedUp) (Variables|Default|GetIsDead) (Variables|Default|GetStaggered) (Variables|Default|GetKnockedOnBack) (Variables|Default|GetDealingDamageIndicator)))
    (Utilities|FlowControl|Gate false :!label _label
      (:Exit
        (Utilities|FlowControl|Sequence
          (:then_0
            (CallFunction|RotatetoFace)
            (Utilities|FlowControl|Delay 0.5)
            (if (not (Math|Boolean|ORBoolean (Variables|Default|GetBeingHitIndicator) (Variables|Default|GetKnockedUp) (Variables|Default|GetIsDead) (Variables|Default|GetStaggered) (Variables|Default|GetKnockedOnBack) (Variables|Default|GetDealingDamageIndicator)))
              (Variables|Default|SetDealingDamageIndicator true)
              (bind _outhit (Collision|SphereTraceForObjects _returnvalue _returnvalue 75.0 (Utilities|Array|MakeArray "ObjectTypeQuery8") false 0 "ForDuration"))
              (bind _asplayer_character (Utilities|Casting|CastToPlayer_Character (.HitActor (Collision|BreakHitResult _outhit)))
                (:then
                  (Default|RecieveDamage _asplayer_character 0.5 (Math|Rotator|GetRotationXVector (Math|Rotator|FindLookatRotation (Transformation|GetActorLocation) (.Location (Collision|BreakHitResult _outhit)))) 5e+01 false false (.Location (Collision|BreakHitResult _outhit)) false false false))
                (:CastFailed
                  _))
              (Utilities|FlowControl|Delay 0.5)
              (Variables|Default|SetDealingDamageIndicator false)))
          (:then_1
            (goto _label Close))
          (:then_2
            (Utilities|FlowControl|Delay 5.0)
            (goto _label Open)))))))

(event EventBeginPlay
  (bind _playerref (Variables|Default|GetPlayerRef))
  (|CallParentFunction)
  ;[1 1 1] UNCONNECTED -WALK TO
  (bind _outhit (Collision|LineTraceForObjects (+ (Transformation|GetActorLocation) "0, 0,50.000000") (+ (Transformation|GetActorLocation _playerref) "0, 0,50.000000") (Utilities|Array|MakeArray "ObjectTypeQuery2") false 0 "None" :!label _label))
  (if (and (<= (Transformation|GetDistanceTo _playerref) 7.5e+02) (not (.bBlockingHit (Collision|BreakHitResult _outhit))))
    (AI|AIMoveTo self "0, 0, 0" (Variables|Default|GetPlayerRef) 5e+01 true
      (:OnSuccess
        (CallFunction|MeleeAttack))
      (:OnFail
        _))
    (Utilities|FlowControl|Delay 2.0)
    (goto _label)
    (else
      (Utilities|FlowControl|Delay 2.5)
      (goto _label))))

(event Collision|EventActorBeginOverlap
  (params (OtherActor :type Actor%20Object%20Reference)))

(event EventTick
  (params (DeltaSeconds :type Float%20%28single-precision%29))
  (|CallParentFunction DeltaSeconds) ; This node is disabled and will not be called.\nDrag off pins to build functionality.
)

(fn ConstructionScript
  (|CallParentFunction))