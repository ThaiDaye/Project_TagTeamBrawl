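; Ranged enemy character that keeps combat distance from the player and fires projectiles.
; A looping BeginPlay chain, not Tick, checks engage range and a WorldDynamic line trace, then uses AIMoveTo to approach, or retreat to a random navigable point when crowded.
; A successful move triggers RangeAttack, which turns to face and, after a wind-up, spawns a projectile unless hit, staggered, downed, dead or already attacking.
; A self-reopening gate provides the attack cooldown.
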(event Custom|RangeAttack
  (CallFunction|RotatetoFace)
  (if (not (Math|Boolean|ORBoolean (Variables|Default|GetBeingHitIndicator) (Variables|Default|GetKnockedUp) (Variables|Default|GetIsDead) (Variables|Default|GetStaggered) (Variables|Default|GetKnockedOnBack) (Variables|Default|GetDealingDamageIndicator)))
    (Utilities|FlowControl|Gate false :!label _label
      (:Exit
        (Utilities|FlowControl|Sequence
          (:then_0
            (Utilities|FlowControl|Delay 1.0)
            (if (not (Math|Boolean|ORBoolean (Variables|Default|GetBeingHitIndicator) (Variables|Default|GetKnockedUp) (Variables|Default|GetIsDead) (Variables|Default|GetStaggered) (Variables|Default|GetKnockedOnBack) (Variables|Default|GetDealingDamageIndicator)))
              (Variables|Default|SetDealingDamageIndicator true)
              (Game|SpawnActorfromClass (Variables|Default|GetProejctile) (Transformation|GetActorTransform) "AlwaysSpawn" 0 0.5 0.5 1e+01 0.5 false 0)
              (Utilities|FlowControl|Delay 1.0)
              (Variables|Default|SetDealingDamageIndicator false)))
          (:then_1
            (goto _label Close))
          (:then_2
            (Utilities|FlowControl|Delay 5.0)
            (goto _label Open)))))))

(event EventBeginPlay
  (bind _returnvalue (Transformation|GetActorLocation))
  (bind _self self)
  (bind _playerref (Variables|Default|GetPlayerRef))
  (|CallParentFunction)
  ;[1 1 1] UNCONNECTED -WALK TO
  (bind _outhit (Collision|LineTraceForObjects (+ (Transformation|GetActorLocation) "0, 0,50.000000") (+ (Transformation|GetActorLocation _playerref) "0, 0,50.000000") (Utilities|Array|MakeArray "ObjectTypeQuery2") false 0 "None" :!label _label))
  (if (and (<= (Transformation|GetDistanceTo _playerref) (Variables|Default|GetEngageRange)) (not (.bBlockingHit (Collision|BreakHitResult _outhit))))
    (if (<= (Transformation|GetDistanceTo _playerref) (Variables|Default|GetRetreatTriggerDistance))
      (bind _randomlocation (Class|NavigationSystemV1|GetRandomLocationinNavigableRadius (+ _returnvalue (* (Math|Rotator|GetRotationXVector (Math|Rotator|FindLookatRotation (Transformation|GetActorLocation _playerref) _returnvalue)) (Variables|Default|GetRetreatDistance))) (Variables|Default|GetRetreatRadius) 0 0))
      (AI|AIMoveTo _self _randomlocation 0 5e+01 true
        (:OnSuccess
          (CallFunction|RangeAttack :!label _label_2))
        (:OnFail
          _))
      (else
        (AI|AIMoveTo _self "0, 0, 0" (Variables|Default|GetPlayerRef) (Variables|Default|GetCombatRange) true
          (:OnSuccess
            (goto _label_2))
          (:OnFail
            _))))
    (Utilities|FlowControl|Delay 1.0)
    (goto _label)
    (else
      (Utilities|FlowControl|Delay 2.5)
      (goto _label))))

(event Collision|EventActorBeginOverlap
  (params (OtherActor :type Actor%20Object%20Reference)))

(event EventTick
  (params (DeltaSeconds :type Float%20%28single-precision%29))
  (|CallParentFunction DeltaSeconds) ; This node is disabled and will not be called.\nDrag off pins to build functionality.
)

(fn ConstructionScript
  (|CallParentFunction))