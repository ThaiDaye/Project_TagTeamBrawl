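; Master projectile that flies by a looping-timer local X offset, gated so it stops on impact and can resume via ReApplyVelocity.
; On hitting a Character_MASTER, it sphere-traces along the inverse hit normal to snap onto the surface and attaches at the hit bone.
; It then applies damage, stagger and knock-up options and disables collision.
; A second timer destroys planted projectiles whose target is no longer valid.
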(event Custom|CullPlantedProjectiles
  (if (Variables|Default|GetPlanted)
    (Utilities|IsValid (Variables|Default|GetPlantedTarget)
      (:Is%20Not%20Valid
        (Actor|DestroyActor)))))

(event Custom|ApplyVelocity
  (Utilities|FlowControl|Gate false
    (:Exit
      (Transformation|AddActorLocalOffset (Math|Vector|MakeVector (Variables|Default|GetVelocity) 0.0 0.0) false false))))

(event Custom|ReApplyVelocity
  (Utilities|FlowControl|Gate false) ; enters at Open
)

(event EventBeginPlay
  (bind _outactors (Actor|GetAllActorsOfClass "/Game/Blueprints/Player_Character.Player_Character_C"))
  (Variables|Default|SetPlayerRef (Utilities|Array|Get(acopy) _outactors))
  (Utilities|Time|SetTimerbyEvent (delegate Custom|ApplyVelocity) 0.001 true)
  (Utilities|Time|SetTimerbyEvent (delegate Custom|CullPlantedProjectiles) 0.1 true))

(event Collision|EventHit
  (params (MyComp :type Primitive%20Component%20Object%20Reference) (Other :type Actor%20Object%20Reference) (OtherComp :type Primitive%20Component%20Object%20Reference) (bSelfMoved :type Boolean) (HitLocation :type Vector :default "0, 0, 0") (HitNormal :type Vector :default "0, 0, 0") (NormalImpulse :type Vector :default "0, 0, 0") (Hit :type Hit%20Result%20Structure%20%28by%20ref%29))
  (bind (_bblockinghit _binitialoverlap _time _distance _location _impactpoint _normal _impactnormal _physmat _hitactor _hitcomponent _hitbonename) (Collision|BreakHitResult Hit))
  (if (not (Variables|Default|GetPlanted))
    (Utilities|FlowControl|Sequence
      (:then_0
        (Utilities|FlowControl|Gate false) ; enters at Close
      )
      (:then_1
        (bind _ascharacter_master (Utilities|Casting|CastToCharacter_MASTER Other))
        (bind _outhit (Collision|SphereTraceForObjects _impactpoint (+ _impactpoint (* _normal -1e+02)) 15.0 (Utilities|Array|MakeArray "ObjectTypeQuery1" "ObjectTypeQuery4" "ObjectTypeQuery2" "ObjectTypeQuery8") false 0 "None"))
        (if (.bBlockingHit (Collision|BreakHitResult _outhit))
          (Transformation|SetActorLocation (.ImpactPoint (Collision|BreakHitResult _outhit)) false false))
        (Transformation|AttachComponentToComponent (Variables|/Script/Engine.Character|GetMesh _ascharacter_master) _hitbonename "KeepWorld" "KeepWorld" "KeepWorld" false)
        (Default|RecieveDamage _ascharacter_master (Variables|Default|GetProjectile%20Damage) (* (.Normal (Collision|BreakHitResult _outhit)) -1.0) (Variables|Default|GetProjectile%20Stagger) (Variables|Default|GetCanKnockup) false (.ImpactPoint (Collision|BreakHitResult _outhit)) (Variables|Default|GetDoesntTriggerOnHit))
        (Variables|Default|SetPlantedTarget _ascharacter_master)
        (Variables|Default|SetPlanted true)
        (Collision|SetCollisionEnabled (Variables|Default|GetBox) "NoCollision")))))

(fn ConstructionScript)