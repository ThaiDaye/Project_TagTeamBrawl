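; Base character Blueprint with the combat logic shared by players and enemies: damage, hit reactions, death, combo counting and attack telegraphs.
; RecieveDamage applies armor and i-frames, then drives stagger, knock-up, damage numbers, camera shake and Death.
; Casts to Enemy_Character and Player_Character add combo hits, Gravity Archer arrow returns and homing shots, and Demon Hammer chilled executes.
; Stagger uses a swept timeline push, and death waits out hit reactions.
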(event Custom|TriggerStagger
  (params (HitDirection :type Vector) (StaggerAmount :type Float%20%28single-precision%29))
  ;[1 1 1] STAGGER
  (Development|PrintString "STAGGER")
  (Variables|Default|SetStaggered true)
  (Animation|PlayAnimMontage (Utilities|Select :Index (Math|Random|RandomIntegerinRange 0 2) :Option%200 "/Game/Geometry/Mannequin/Animations/Animations_Action/12_Frank_Hit_high_Inplace_Montage.12_Frank_Hit_high_Inplace_Montage" :Option%201 "/Game/Geometry/Mannequin/Animations/Animations_Action/13_Frank_Hit_Middle_Inplace_Montage.13_Frank_Hit_Middle_Inplace_Montage" :Option%202 "/Game/Geometry/Mannequin/Animations/Animations_Action/14_Frank_Hit_Heavy_Inplace_Montage.14_Frank_Hit_Heavy_Inplace_Montage") 1.0 "None")
  (Variables|Default|SetBeforeHitLocation (Transformation|GetActorLocation))
  (bind _newtrack_0 (Timeline|Timeline_0 PlayFromStart)
    (:Update
      (Transformation|SetActorLocation (Math|Vector|Lerp(Vector) (Variables|Default|GetBeforeHitLocation) (Math|Vector|MakeVector (.x (+ (* HitDirection StaggerAmount) (Variables|Default|GetBeforeHitLocation))) (.y (+ (* HitDirection StaggerAmount) (Variables|Default|GetBeforeHitLocation))) (.Z (Math|Vector|BreakVector (Variables|Default|GetBeforeHitLocation)))) _newtrack_0) true false))
    (:Finished
      (Utilities|FlowControl|Delay (Variables|Default|GetStaggerDelay))
      (Variables|Default|SetStaggered false))))

(event Custom|Death
  (params (IsDead :type Boolean) (ChilledKill :type Boolean) (Executed :type Boolean))
  (bind _capsulecomponent (Variables|Collision|GetCapsuleComponent))
  (if IsDead
    (Variables|Default|SetIsDead true)
    (CallFunction|GravityArcherSpawnReturnGravArrow 3)
    (if Executed
      (Variables|Default|SetHealth 0.0)
      (bind _asenemy_character (Utilities|Casting|CastToEnemy_Character self)
        (:then
          (Default|DemonHammerMobilityResetCooldown (Variables|/Game/Blueprints/Enemies/Enemy_Character.Enemy_Character_C|GetPlayerRef _asenemy_character)))
        (:CastFailed
          _)))
    (if ChilledKill
      (Game|SpawnActorfromClass "/Game/Blueprints/StaticEntities/StaticEntity_DemonHammerIcecile.StaticEntity_DemonHammerIcecile_C" (Transformation|GetActorTransform) "AlwaysSpawn" 0 0)
      (Actor|DestroyActor)
      (else
        (if (or (Variables|Default|GetBeingHitIndicator) (Variables|Default|GetKnockedUp)) :!label _label
          (Utilities|FlowControl|Delay 0.05)
          (goto _label)
          (else
            (Development|PrintString "DEAD")
            (if (Variables|Default|GetKnockedOnBack)
              (Actor|DestroyActor)
              (else
                (Collision|SetCollisionResponsetoAllChannels _capsulecomponent "ECR_Ignore")
                (Collision|SetCollisionResponsetoChannel _capsulecomponent "ECC_WorldStatic" "ECR_Block")
                (Animation|PlayAnimMontage "/Game/Geometry/Mannequin/Animations/Animations_Action/17_Frank_Hit_KnockDown_Inplace_Montage.17_Frank_Hit_KnockDown_Inplace_Montage" 1.0 "None")))))))))

(event Custom|Effect-KnockUp
  (Variables|Default|SetKnockedUp true)
  (Development|PrintString "KNOCKUP")
  (Animation|PlayAnimMontage "/Game/Geometry/Mannequin/Animations/Animations_Action/15_Frank_Hit_Air_Inplace_Montage.15_Frank_Hit_Air_Inplace_Montage" 1.0 "None"))

(event Custom|TriggerIFrame
  (Utilities|FlowControl|RetriggerableDelay (Variables|Default|GetBeingHitIFrames))
  (Variables|Default|SetBeingHitIndicator false))

(event Custom|Effect-KnockUpEnd
  (Variables|Default|SetKnockedUp false))

(event Custom|GravityArcher_SpawnReturnGravArrow
  (params (AddArrows :type Integer))
  (bind _self self)
  (bind _asenemy_character (Utilities|Casting|CastToEnemy_Character _self)
    (:then
      (if (> (Variables|/Game/Blueprints/Enemies/Enemy_Character.Enemy_Character_C|GetGravityArrowCount _asenemy_character) 0)
        (for _index (range 1 (Math|Integer|Clamp(Integer) AddArrows 0 (Variables|/Game/Blueprints/Enemies/Enemy_Character.Enemy_Character_C|GetGravityArrowCount _asenemy_character)))
          (Game|SpawnActorfromClass "/Game/Blueprints/StaticEntities/StaticEntity_ReturningGravArrow.StaticEntity_ReturningGravArrow_C" (Math|Transform|MakeTransform (Transformation|GetActorLocation _asenemy_character) "0, 0, 0" "1,1,1") "AlwaysSpawn" 0 false 0))
        (Variables|/Game/Blueprints/Enemies/Enemy_Character.Enemy_Character_C|SetGravityArrowCount _asenemy_character (Math|Integer|Clamp(Integer) (- (Variables|/Game/Blueprints/Enemies/Enemy_Character.Enemy_Character_C|GetGravityArrowCount _asenemy_character) AddArrows) 0 (Variables|/Game/Blueprints/Enemies/Enemy_Character.Enemy_Character_C|GetGravityArrowCount _asenemy_character)))))
    (:CastFailed
      (bind _asplayer_character (Utilities|Casting|CastToPlayer_Character _self))
      (for _index_2 (range 1 AddArrows)
        (Game|SpawnActorfromClass "/Game/Blueprints/StaticEntities/StaticEntity_ReturningGravArrow.StaticEntity_ReturningGravArrow_C" (Math|Transform|MakeTransform (Transformation|GetActorLocation _asplayer_character) "0, 0, 0" "1,1,1") "AlwaysSpawn" 0 true 0))
      (Variables|/Game/Blueprints/Player_Character.Player_Character_C|SetGravityArcher_GravArrowCount _asplayer_character (+ (Variables|/Game/Blueprints/Player_Character.Player_Character_C|GetGravityArcher_GravArrowCount _asplayer_character) AddArrows)))))

(event Custom|AddToAttackCombo
  (Utilities|FlowControl|Gate false :!label _label
    (:Exit
      (Utilities|FlowControl|Sequence
        (:then_0
          (Variables|Default|SetComboHitCounter (+ (Variables|Default|GetComboHitCounter) 1))
          (Variables|Default|SetComboHitDuration (Variables|Default|GetComboHitDurationMax))
          (if (== (Variables|Default|GetComboHitDuration) 0.0) :!label _label_2
            (Variables|Default|SetComboHitCounter 0)
            (else
              (Utilities|FlowControl|RetriggerableDelay 0.1)
              (goto _label_2))))
        (:then_1
          (goto _label Close))
        (:then_2
          (Utilities|FlowControl|Delay 0.1)
          (goto _label Open))))))

(event Custom|ComboHitCooldown
  (Variables|Default|SetComboHitDuration (Math|Float|Clamp(Float) (- (Variables|Default|GetComboHitDuration) 0.01) 0.0 (Variables|Default|GetComboHitDurationMax))))

(event Custom|DisplayTelegraph
  (params (Type :type Telegraph_Types%20Enum :default "NewEnumerator0") (Scale%20X :type Float%20%28single-precision%29) (Scale%20Y :type Float%20%28single-precision%29) (AutoDismiss :type Boolean) (AutoDismissDelay :type Float%20%28single-precision%29) (CenterOnZero :type Boolean) (DontMovePivot :type Boolean))
  (bind _telegraph (Variables|Default|GetTelegraph))
  (if DontMovePivot
    _
    (else
      (Transformation|SetRelativeLocation (Variables|Default|GetTelegraph) (select CenterOnZero "0, 0, 0" "-30.000000, 0, 0") false false)))
  (Transformation|SetRelativeScale3D _telegraph (Math|Vector|MakeVector Scale%20X Scale%20Y 1e+01))
  (Components|StaticMesh|SetStaticMesh _telegraph (Utilities|Select :Index Type :NewEnumerator0 "/Game/Geometry/Meshes/Telegraph_Box.Telegraph_Box" :NewEnumerator1 "/Engine/BasicShapes/Cylinder.Cylinder" :NewEnumerator2 "/Game/Geometry/Meshes/Telegraph_180.Telegraph_180" :NewEnumerator3 "/Game/Geometry/Meshes/Telegraph_90.Telegraph_90" :NewEnumerator4 "/Game/Geometry/Meshes/Telegraph_40.Telegraph_40"))
  (Rendering|SetVisibility _telegraph true false)
  (if AutoDismiss
    (Utilities|FlowControl|RetriggerableDelay AutoDismissDelay)
    (CallFunction|DismissTelegraph)))

(event Custom|DismissTelegraph
  (Rendering|SetVisibility (Variables|Default|GetTelegraph) false false))

(event EventBeginPlay
  (Utilities|Time|SetTimerbyEvent (delegate Custom|ComboHitCooldown) 0.01 true))

(fn ConstructionScript)

(fn RecieveDamage
  (params (damage :type Float%20%28single-precision%29) (HitDirection :type Vector) (stagger%20amount :type Float%20%28single-precision%29) (KnockUp :type Boolean) (ChipDamage :type Boolean) (HitLocation :type Vector) (DontTriggerOnHit :type Boolean) (ChilledKill :type Boolean) (ExecuteKill :type Boolean))
  (bind _armorvalue (Variables|Default|GetArmorValue))
  (bind _returnvalue (- _armorvalue 1.0))
  (bind _returnvalue_2 (* _returnvalue damage))
  (bind _returnvalue_3 (- damage _returnvalue_2))
  (if (not (Variables|Default|GetInvunerable))
    (if (not (Variables|Default|GetBeingHitIndicator))
      (Variables|Default|SetBeingHitIndicator true)
      (Development|PrintString "HIT")
      (Variables|Default|SetHealth (Math|Float|Clamp(Float) (- (Variables|Default|GetHealth) _returnvalue_3) 0.0 (Variables|Default|GetMaxhealth)))
      (CallFunction|DismissTelegraph)
      (CallFunction|TriggerStagger HitDirection stagger%20amount)
      (if (== _returnvalue_3 0.0)
        _
        (else
          (Game|SpawnActorfromClass "/Game/Blueprints/UI/DamageIndicator_BP.DamageIndicator_BP_C" (Math|Transform|MakeTransform (select (Math|Vector|Equal(Vector) HitLocation "0, 0, 0" 0.0001) (Transformation|GetActorLocation) HitLocation)) "AlwaysSpawn" 0 _returnvalue_3 0)
          (bind _asenemy_character (Utilities|Casting|CastToEnemy_Character self)
            (:then
              (CallFunction|AddtoAttackCombo (Variables|/Game/Blueprints/Enemies/Enemy_Character.Enemy_Character_C|GetPlayerRef _asenemy_character)))
            (:CastFailed
              _))))
      (if ChipDamage
        (Variables|Default|SetKnockedUp false)
        (else
          (Transformation|SetActorRotation (Math|Rotator|MakeRotator 0.0 0.0 (.yaw (Math|Conversions|RotationFromXVector (* HitDirection -1.0)))))
          (Camera|PlayWorldCameraShake (Variables|Default|GetAttackShake) HitLocation 0.0 1e+05)
          (if (Variables|Default|GetKnockedUp)
            (CallFunction|Effect-KnockUp :!label _label)
            (elif KnockUp
              (goto _label)
              (else
                _)))))
      (CallFunction|TriggerIFrame)
      (bind _asenemy_character_2 (Utilities|Casting|CastToEnemy_Character self)
        (:then
          (if (> (Variables|/Game/Blueprints/Player_Character.Player_Character_C|GetGravityArcher_GravArrowCount (Variables|/Game/Blueprints/Enemies/Enemy_Character.Enemy_Character_C|GetPlayerRef _asenemy_character_2)) 0)
            (if (Variables|Default|GetIsDead)
              _
              (elif DontTriggerOnHit
                _
                (elif ChipDamage
                  _
                  (else
                    (Default|GravityArcherFireHomingArrow (Variables|/Game/Blueprints/Enemies/Enemy_Character.Enemy_Character_C|GetPlayerRef _asenemy_character_2) HitLocation)))))))
        (:CastFailed
          _))
      (bind _asenemy_character_3 (Utilities|Casting|CastToEnemy_Character self)
        (:then
          (CallFunction|Death (select ExecuteKill (<= (/ (Variables|Default|GetHealth) (Variables|Default|GetMaxhealth)) (select (Variables|/Game/Blueprints/Enemies/Enemy_Character.Enemy_Character_C|GetDemonHammer_Chilled _asenemy_character_3) 0.25 0.0)) (<= (Variables|Default|GetHealth) 0.0)) ChilledKill (Math|Boolean|ANDBoolean (<= (/ (Variables|Default|GetHealth) (Variables|Default|GetMaxhealth)) (select (Variables|/Game/Blueprints/Enemies/Enemy_Character.Enemy_Character_C|GetDemonHammer_Chilled _asenemy_character_3) 0.25 0.0)) (Variables|/Game/Blueprints/Enemies/Enemy_Character.Enemy_Character_C|GetDemonHammer_Chilled _asenemy_character_3) ExecuteKill)))
        (:CastFailed
          (CallFunction|Death (<= (Variables|Default|GetHealth) 0.0) false false))))))