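; A tombstone static entity that the player plants in the world and can send back as a returning projectile.
; On BeginPlay it registers itself with the first Player_Character found through TombstonePlant, then sphere-traces around its location to trigger any DesecratedGround entities it lands on.
; ReturnTombstone spawns a ReturningTombstone_projectile at its transform and destroys the tombstone.
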(event Custom|ReturnTombstone
  (Game|SpawnActorfromClass "/Game/Blueprints/Projectiles/ReturningTombstone_projectile.ReturningTombstone_projectile_C" (Transformation|GetActorTransform) "AdjustIfPossibleButAlwaysSpawn" 0 0.0 5e+01 1.0 0)
  (Actor|DestroyActor))

(event EventBeginPlay
  (bind _returnvalue (Transformation|GetActorLocation))
  (|CallParentFunction)
  (bind _outactors (Actor|GetAllActorsOfClass "/Game/Blueprints/Player_Character.Player_Character_C"))
  (bind _output_get (Variables|Default|SetPlayerRef (Utilities|Array|Get(acopy) _outactors)))
  (Default|TombstonePlant _output_get self)
  (bind _outhits (Collision|MultiSphereTraceForObjects _returnvalue _returnvalue 5e+01 (Utilities|Array|MakeArray "ObjectTypeQuery10") false 0 "None"))
  (for _array_element _outhits
    (bind _asstatic_entity_desecrated_ground (Utilities|Casting|CastToStaticEntity_DesecratedGround (.HitActor (Collision|BreakHitResult _array_element))))
    (Default|DesecratedTrigger _asstatic_entity_desecrated_ground)))

(event Collision|EventActorBeginOverlap
  (params (OtherActor :type Actor%20Object%20Reference))
  (|CallParentFunction OtherActor) ; This node is disabled and will not be called.\nDrag off pins to build functionality.
)

(event EventTick
  (params (DeltaSeconds :type Float%20%28single-precision%29))
  (|CallParentFunction DeltaSeconds) ; This node is disabled and will not be called.\nDrag off pins to build functionality.
)

(fn ConstructionScript
  (|CallParentFunction))