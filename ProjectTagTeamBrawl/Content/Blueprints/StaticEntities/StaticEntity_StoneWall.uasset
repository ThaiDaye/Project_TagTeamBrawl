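; Stone wall static entity that acts as a temporary barrier, destroying itself after a fixed delay.
; On BeginPlay it caches the first Player_Character and attaches its mesh to a SpringArm, keeping world transform.
; Every tick, enemies overlapping the mesh take staggering chip damage directed away from the wall.
; Hit events pass the other object to the player's DeflectProjectile as a projectile.
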(event EventBeginPlay
  (|CallParentFunction)
  (bind _outactors (Actor|GetAllActorsOfClass "/Game/Blueprints/Player_Character.Player_Character_C"))
  (Variables|Default|SetPlayerRef (Utilities|Array|Get(acopy) _outactors))
  (Transformation|AttachComponentToComponent (Variables|Default|GetStaticMesh) (Variables|Default|GetSpringArm) "None" "KeepWorld" "KeepWorld" "KeepWorld" true)
  (Utilities|FlowControl|Delay 1e+01)
  (Actor|DestroyActor))

(event EventTick
  (params (DeltaSeconds :type Float%20%28single-precision%29))
  (bind _returnvalue (Transformation|GetActorLocation))
  (|CallParentFunction DeltaSeconds)
  (for _array_element (Collision|GetOverlappingActors (Variables|Default|GetStaticMesh) "/Game/Blueprints/Enemies/Enemy_Character.Enemy_Character_C" :!class /Script/Engine.PrimitiveComponent)
    (bind _asenemy_character (Utilities|Casting|CastToEnemy_Character _array_element))
    (Default|RecieveDamage _asenemy_character 0.0 (Math|Rotator|GetRotationXVector (Math|Rotator|FindLookatRotation (Math|Vector|MakeVector (.x _returnvalue) (.y _returnvalue) 0.0) (Math|Vector|MakeVector (.x (Transformation|GetActorLocation _asenemy_character)) (.y (Transformation|GetActorLocation _asenemy_character)) 0.0))) 1e+02 false true (Transformation|GetActorLocation _asenemy_character) false false false)))

(event Collision|EventHit
  (params (MyComp :type Primitive%20Component%20Object%20Reference) (Other :type Actor%20Object%20Reference) (OtherComp :type Primitive%20Component%20Object%20Reference) (bSelfMoved :type Boolean) (HitLocation :type Vector :default "0, 0, 0") (HitNormal :type Vector :default "0, 0, 0") (NormalImpulse :type Vector :default "0, 0, 0") (Hit :type Hit%20Result%20Structure%20%28by%20ref%29))
  (Default|DeflectProjectile (Variables|Default|GetPlayerRef) Other HitLocation))

(fn ConstructionScript
  (|CallParentFunction))