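; Static entity for a gravity arrow that flies back to the player character to replenish the Gravity Archer's arrow count.
; On BeginPlay it waits a random delay unless quick return is set, then a timeline moves it along a randomized sideways and upward arc toward the player's live position while facing them.
; On arrival it increments the clamped count, spawns a hovering arrow inside the player's ArrowBox, registers it, and destroys itself.
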(event Custom|ReturnArrow
  (bind _playerref (Variables|Default|GetPlayerRef))
  (bind _playerref_2 (Variables|Default|GetPlayerRef))
  (bind _returnvalue (Transformation|GetActorLocation _playerref_2))
  (bind _arrowbox (Variables|/Game/Blueprints/Player_Character.Player_Character_C|GetArrowBox _playerref))
  (Variables|Default|SetStartLocation (Transformation|GetActorLocation))
  (bind _output_get (Variables|Default|SetNewVar_0 (Math|Random|RandomFloatinRange 0.0 1.0)))
  (bind _output_get_2 (Variables|Default|SetNewVar_1 (Math|Random|RandomFloatinRange 0.0 1.0)))
  (bind (_direction _newtrack_0 _newtrack_1) (Timeline|Timeline_0 PlayFromStart)
    (:Update
      (Transformation|SetActorLocation (+ (Math|Vector|Lerp(Vector) (Variables|Default|GetStartLocation) _returnvalue _newtrack_0) (Math|Vector|Lerp(Vector) "0, 0, 0" (+ (* (Math|Vector|GetRightVector (Math|Rotator|FindLookatRotation (Variables|Default|GetStartLocation) _returnvalue)) (Math|Float|Lerp -5e+02 5e+02 _output_get)) (Math|Vector|MakeVector 0.0 0.0 (Math|Float|Lerp 1e+02 5e+02 _output_get_2))) _newtrack_1)) false false)
      (Transformation|SetActorRotation (Math|Rotator|FindLookatRotation (Transformation|GetActorLocation) (Transformation|GetActorLocation (Variables|Default|GetPlayerRef)))))
    (:Finished
      (Variables|/Game/Blueprints/Player_Character.Player_Character_C|SetGravityArcher_GravArrowCount _playerref (Math|Integer|Clamp(Integer) (+ (Variables|/Game/Blueprints/Player_Character.Player_Character_C|GetGravityArcher_GravArrowCount _playerref) 1) 0 100))
      (bind _returnvalue_2 (Game|SpawnActorfromClass "/Game/Blueprints/StaticEntities/StaticEntity_HoveringGravArrow.StaticEntity_HoveringGravArrow_C" (Math|Transform|MakeTransform (Math|Random|RandomPointinBoundingBox (Transformation|GetWorldLocation _arrowbox) (Variables|/Script/Engine.BoxComponent|GetBoxExtent _arrowbox)) (Transformation|GetWorldRotation _arrowbox)) "AlwaysSpawn" 0 0))
      (Transformation|AttachComponentToComponent _returnvalue_2 _arrowbox "None" "KeepWorld" "KeepWorld" "KeepWorld" true)
      (Utilities|Array|Add (Variables|/Game/Blueprints/Player_Character.Player_Character_C|GetGravArrowRefs _playerref) _returnvalue_2)
      (Actor|DestroyActor))))

(event EventBeginPlay
  (|CallParentFunction)
  (bind _outactors (Actor|GetAllActorsOfClass "/Game/Blueprints/Player_Character.Player_Character_C"))
  (Variables|Default|SetPlayerRef (Utilities|Array|Get(acopy) _outactors))
  (if (Variables|Default|GetQucikReturn)
    _
    (else
      (Utilities|FlowControl|Delay (Math|Random|RandomFloatinRange 0.0 1.0))))
  (CallFunction|ReturnArrow))

(fn ConstructionScript
  (|CallParentFunction))