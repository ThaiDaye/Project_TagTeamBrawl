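; Static entity for desecrated ground, a temporary area hazard that damages enemies inside its sphere once triggered.
; A looping one-second timer, started shortly after spawn, applies chip damage and stagger to overlapping enemies while active, with hit direction pointing away from the center.
; DesecratedTrigger activates it and reveals a second sphere.
; Spawn and trigger share a retriggerable ten-second delay before destruction, so triggering restarts the lifetime.
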(event Custom|TickDamage
  (bind _returnvalue (Transformation|GetActorLocation))
  (if (Variables|Default|GetActive)
    (for _array_element (Collision|GetOverlappingActors (Variables|Default|GetSphere) "/Game/Blueprints/Enemies/Enemy_Character.Enemy_Character_C" :!class /Script/Engine.PrimitiveComponent)
      (Utilities|IsValid _array_element
        (:Is%20Valid
          (Default|RecieveDamage (.AsEnemy%20Character (Utilities|Casting|CastToEnemy_Character _array_element)) (Variables|Default|GetProjectile%20Damage) (Math|Rotator|GetRotationXVector (Math|Rotator|FindLookatRotation (Math|Vector|MakeVector (.x _returnvalue) (.y _returnvalue) 0.0) (Math|Vector|MakeVector (.x (Transformation|GetActorLocation _array_element)) (.y (Transformation|GetActorLocation _array_element)) 0.0))) (Variables|Default|GetProjectile%20Stagger) false true (Transformation|GetActorLocation (.AsEnemy%20Character (Utilities|Casting|CastToEnemy_Character _array_element))) false))))))

(event Custom|DesecratedTrigger
  (Development|PrintString "DESECRATED GROUND ACTIVATED")
  (Rendering|SetVisibility (Variables|Default|GetSphere1) true false)
  (Variables|Default|SetActive true)
  (Utilities|FlowControl|RetriggerableDelay 1e+01)
  (Actor|DestroyActor))

(event Collision|EventActorBeginOverlap
  (params (OtherActor :type Actor%20Object%20Reference))
  (|CallParentFunction OtherActor) ; This node is disabled and will not be called.\nDrag off pins to build functionality.
)

(event EventTick
  (params (DeltaSeconds :type Float%20%28single-precision%29))
  (|CallParentFunction DeltaSeconds) ; This node is disabled and will not be called.\nDrag off pins to build functionality.
)

(event EventBeginPlay
  (|CallParentFunction)
  (Utilities|FlowControl|Sequence
    (:then_0
      (Utilities|FlowControl|Delay 0.2)
      (Utilities|Time|SetTimerbyEvent (delegate Custom|TickDamage) 1.0 true))
    (:then_1
      (Utilities|FlowControl|RetriggerableDelay 1e+01)
      (Actor|DestroyActor))))

(fn ConstructionScript
  (|CallParentFunction))